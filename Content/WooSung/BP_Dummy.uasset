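; BP_Dummy is a damageable dummy character that reacts to hits and dies when its health runs out.
; It fills CurrentHp from MaxHp at BeginPlay and subtracts incoming point damage, ignoring hits once health is depleted.
; Surviving hits play an impact sound and hit montage.
; A lethal hit plays an assassination death montage, waits for its returned duration, then destroys the actor.
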(event Custom|PerformHitReaction
  (Audio|PlaySoundatLocation "/Game/CombatSystem/CourseFiles/SoundFX/Gruntling/A_Guardian_Impact01.A_Guardian_Impact01" (Transformation|GetActorLocation) "0, 0, 0" 1.0 1.0 0.0 0 0 0 0)
  (Animation|PlayAnimMontage "/Game/WooSung/Animations/M_HitImpact.M_HitImpact" 1.0 "None"))

(event Custom|Death
  (bind _returnvalue (Animation|PlayAnimMontage "/Game/YEJ/Retargeting-5/Flexible-5/Animation/AssasinationDeath_Montage.AssasinationDeath_Montage" 1.0 "None"))
  (Utilities|FlowControl|Delay _returnvalue)
  (Actor|DestroyActor))

(event EventBeginPlay
  (Variables|Default|SetcurrentHp (Variables|Default|GetmaxHp)))

(event Collision|EventActorBeginOverlap
  (params (OtherActor :type Actor%20Object%20Reference)))

(event EventTick
  (params (DeltaSeconds :type Float%20%28single-precision%29)))

(event Game|Damage|EventPointDamage
  (params (Damage :type Float%20%28single-precision%29) (DamageType :type Damage%20Type%20Object%20Reference) (HitLocation :type Vector :default "0, 0, 0") (HitNormal :type Vector :default "0, 0, 0") (HitComponent :type Primitive%20Component%20Object%20Reference) (BoneName :type Name :default "None") (ShotFromDirection :type Vector :default "0, 0, 0") (InstigatedBy :type Controller%20Object%20Reference) (DamageCauser :type Actor%20Object%20Reference) (HitInfo :type Hit%20Result%20Structure%20%28by%20ref%29))
  (if (not (<= (Variables|Default|GetcurrentHp) 0.0))
    (Variables|Default|SetcurrentHp (- (Variables|Default|GetcurrentHp) Damage))
    (if (> (Variables|Default|GetcurrentHp) 0.0)
      (CallFunction|PerformHitReaction)
      (else
        (CallFunction|Death)))))

(fn ConstructionScript)