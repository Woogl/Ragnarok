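; Test dummy character for the combat system that carries stats, wears starting equipment and can be locked on to.
; On BeginPlay it initializes StatsComp, spawns each StartingEquipment class with itself as owner and instigator, equips it, then prints one current stat.
; The OnTargeted event shows or hides LockOnWidget according to whether the dummy is targeted.
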(event EventBeginPlay
  (bind _self self)
  (Default|InitializeStat (Variables|Default|GetStatsComp)) ; 기본 스탯 설정
  (for _array_element (Variables|Default|GetStartingEquipment) ; 디폴트의 기본 방어구 탐색
    (bind _returnvalue (Game|SpawnActorfromClass _array_element (Transformation|GetActorTransform) "Undefined" _self _self)) ; 방어구 스폰
    (Default|OnEquipped _returnvalue) ; 방어구 장착
  )
  ;[1 1 1] Comment
  (Development|PrintString (Utilities|String|ToString(Float) (Default|GetCurrentStat (Variables|Default|GetStatsComp) "NewEnumerator3"))))

(event EventOnTargeted
  (params (bIsTargeted? :type Boolean))
  ;[0 0 0] 락온
  (Rendering|SetVisibility (Variables|Default|GetLockOnWidget) bIsTargeted? false))

(fn ConstructionScript
  (|CallParentFunction))