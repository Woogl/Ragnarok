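; Player combat character Blueprint that handles movement speed, jumping, dodging, interaction, combo attacks, weapon draw/sheathe, damage and death.
; StateManagerComp gates actions by state, while CombatComp supplies the main weapon, whose montages drive attacks, dodges and combat toggling.
; Attack presses during a swing are buffered, then consumed by anim-notify callbacks that continue or reset the combo.
; Point damage triggers effects and hit reactions; zero health sets Dead, causing ragdoll and delayed destruction.
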(event OnStateBegin(StateManagerComp)
  (params (CharacterState :type ECharacterState%20Enum :default "Nothing"))
  ;[0 0 0] 플레이어 State
  (switch Utilities|FlowControl|Switch|SwitchonECharacterState CharacterState ; C++ Enum
    (:Dead
      (CallFunction|PerformDeath) ; 사망 이벤트로
    )))

(event OnStateEnd(StateManagerComp)
  (params (CharacterState :type ECharacterState%20Enum :default "Nothing"))
  ;[0 0 0] 플레이어 State
  (switch Utilities|FlowControl|Switch|SwitchonECharacterState CharacterState) ; C++ Enum
)

(event OnCharacterActionBegin(StateManagerComp)
  (params (Action :type ECharacterAction%20Enum :default "Nothing"))
  ;[0 0 0] 플레이어 Action
  (switch Utilities|FlowControl|Switch|SwitchonECharacterAction Action))

(event OnCharacterActionEnd(StateManagerComp)
  (params (Action :type ECharacterAction%20Enum :default "Nothing"))
  ;[0 0 0] 플레이어 Action
  (switch Utilities|FlowControl|Switch|SwitchonECharacterAction Action))

(event Custom|AttackEvent
  ;[0 0 0] 공격
  (if (CallFunction|CanPerformAttack?)
    (CallFunction|PerformAttack "GeneralAction" "GeneralActionState" (Variables|/Game/CombatSystem/Blueprints/Components/BP_CombatComp.BP_CombatComp_C|GetAttackCount (Variables|Default|GetCombatComp)) false) ; 3. 몽타주를 선택하고 재생하는 함수를 만듦
  ))

(event Custom|TakeDamage
  (params (In%20Damage :type Float%20%28double-precision%29))
  ;[0 0 0] 피격
  (bind _output_get (Variables|Default|SetHealth (Math|Float|Clamp(Float) (- (Variables|Default|GetHealth) In%20Damage) 0.0 (- (Variables|Default|GetHealth) In%20Damage))))
  (if (<= _output_get 0.0) ; Health 0 이하면 사망
    (Default|SetState (Variables|Default|GetStateManagerComp) "Dead")))

(event Custom|PerformDeath
  (bind _combatcomp (Variables|Default|GetCombatComp))
  (bind _mainweapon (Default|GetMainWeapon _combatcomp))
  ;[0 0 0] 사망
  (CallFunction|EnableRagdoll) ; 래그돌 일어나게
  (CallFunction|ApplyHitReactionPhysicsVelocity 2e+02) ; 캐릭터가 뒤로 밀리게
  (Utilities|FlowControl|Sequence
    (:then_0
      (Utilities|IsValid _mainweapon
        (:Is%20Valid
          (Default|SimulateWeaponPhysics _mainweapon))))
    (:then_1
      (Utilities|FlowControl|Delay 4.0)
      (Utilities|IsValid _mainweapon
        (:Is%20Valid
          (Actor|DestroyActor _mainweapon) ; 무기 파괴
        )
        (:Is%20Not%20Valid
          _))
      (Actor|DestroyActor) ; 캐릭터 파괴
    )))

(event Custom|ToggleCombat
  ;[0 0 0] 무기 꺼내기 / 집어넣기
  (if (CallFunction|CanPerformToggleCombat?)
    (Default|SetState (Variables|Default|GetStateManagerComp) "GeneralActionState")
    (if (not (Default|IsCombatEnabled? (Variables|Default|GetCombatComp))) ; 4. 무기 꺼내놓은 상태인가?
      (CallFunction|PerformAction (Utilities|Array|MakeArray (Variables|/Game/CombatSystem/Blueprints/Actors/BP_BaseWeapon.BP_BaseWeapon_C|GetEnterCombat (Default|GetMainWeapon (Variables|Default|GetCombatComp)))) "EnterCombat" "GeneralActionState" 0 false)
      (else
        (CallFunction|PerformAction (Utilities|Array|MakeArray (Variables|/Game/CombatSystem/Blueprints/Actors/BP_BaseWeapon.BP_BaseWeapon_C|GetExitCombat (Default|GetMainWeapon (Variables|Default|GetCombatComp)))) "ExitCombat" "GeneralActionState" 0 false)))))

(event Custom|DodgeEvent
  ;[0 0 0] 회피
  (if (CallFunction|CanPerformDodge?)
    (CallFunction|PerformDodge 0 false) ; 몽타주 선택하고 재생하는 함수를 만듦
  ))

(event EventBeginPlay
  ;[1 1 1] Begin Play
)

(event EventContinueAttack
  (bind _combatcomp (Variables|Default|GetCombatComp))
  ;[0 0 0] Anim Notify 이벤트
  (Default|SetState (Variables|Default|GetStateManagerComp) "Attacking")
  (if (Variables|/Game/CombatSystem/Blueprints/Components/BP_CombatComp.BP_CombatComp_C|GetbIsAttackSaved? _combatcomp) ; 2. 다음 공격 입력했는지 플래그 체크
    (Variables|/Game/CombatSystem/Blueprints/Components/BP_CombatComp.BP_CombatComp_C|SetbIsAttackSaved? _combatcomp false)
    (if (Utilities|Enum|Equal(Enum) (Default|GetCurrentState (Variables|Default|GetStateManagerComp)) "Attacking") ; State 체크
      (Default|SetState (Variables|Default|GetStateManagerComp) "Nothing"))
    (CallFunction|AttackEvent) ; 3. 다음 공격 콤보도 실행
  ))

(event EventResetAttack
  ;[0 0 0] Anim Notify 이벤트
  (Default|ResetAttack (Variables|Default|GetCombatComp)))

(event EventResetCombat
  ;[0 0 0] Anim Notify 이벤트
  (Default|ResetAttack (Variables|Default|GetCombatComp))
  (Default|ResetState (Variables|Default|GetStateManagerComp)) ; State를 Nothing으로 바꿈
  (Default|SetCurrentAction (Variables|Default|GetStateManagerComp) "Nothing") ; Nothing
)

(event Game|Damage|EventPointDamage
  (params (Damage :type Float%20%28single-precision%29) (DamageType :type Damage%20Type%20Object%20Reference) (HitLocation :type Vector :default "0, 0, 0") (HitNormal :type Vector :default "0, 0, 0") (HitComponent :type Primitive%20Component%20Object%20Reference) (BoneName :type Name :default "None") (ShotFromDirection :type Vector :default "0, 0, 0") (InstigatedBy :type Controller%20Object%20Reference) (DamageCauser :type Actor%20Object%20Reference) (HitInfo :type Hit%20Result%20Structure%20%28by%20ref%29))
  ;[0 0 0] 피격
  (CallFunction|TakeDamage Damage)
  (Development|PrintString (Utilities|String|Append (Utilities|String|ToString(Float) Damage) "points of damage was applied by " "Damage Causer : " (Utilities|GetDisplayName DamageCauser) "Instigator : " (Utilities|GetDisplayName (Pawn|GetControlledPawn InstigatedBy))) true true "(R=0.000000,G=0.660000,B=1.000000,A=1.000000)" 5.0)
  (Audio|PlaySoundatLocation "/Game/CombatSystem/CourseFiles/SoundFX/Gruntling/A_Guardian_Impact01_Cue.A_Guardian_Impact01_Cue" HitLocation "0, 0, 0" 1.0 1.0 0.0 0 0 0 0) ; 타격 SFX
  (Effects|SpawnEmitteratLocation "/Game/VFX/Realistic_Starter_VFX_Pack_Vol2/Particles/Blood/P_Blood_Splat_Cone.P_Blood_Splat_Cone" HitLocation) ; 피 VFX
  (if (CallFunction|CanReceiveHitReaction?) ; Dead 상태는 HitReaction 없음
    (Default|SetState (Variables|Default|GetStateManagerComp) "Disabled") ; 이동 불가 상태
    (Animation|PlayAnimMontage "/Game/CombatSystem/CourseFiles/Animations/HitReactions/Standing_React_Large_Front_Montage.Standing_React_Large_Front_Montage" 1.0 "None")))

(event EventMyJump
  ;[0 0 0] 점프
  (if (CallFunction|CanJump?)
    (Animation|StopAnimMontage 0) ; 재생 중이던 애니메이션 캔슬
    (Default|ResetState (Variables|Default|GetStateManagerComp))
    (Character|Jump)))

(event Input|ActionEvents|InputActionToggleCombat
  (params (Key :type Key%20Structure :default "None"))
  ;[0 0 0] 무기 꺼내기 / 집어넣기
  (:Pressed
    (Utilities|IsValid (Default|GetMainWeapon (Variables|Default|GetCombatComp)) ; 2. 무기 있을 때만 실행
      (:Is%20Valid
        (CallFunction|ToggleCombat)))))

(event Input|ActionEvents|InputActionInteract
  (params (Key :type Key%20Structure :default "None"))
  (bind _returnvalue (Transformation|GetActorLocation))
  ;[0 0 0] 상호작용
  (:Pressed
    (bind (_outhit _returnvalue_2) (Collision|SphereTraceForObjects _returnvalue _returnvalue 1e+02 (Utilities|Array|MakeArray "ObjectTypeQuery7") false (Utilities|Array|MakeArray self) "None")) ; WorldDynamic 오브젝트를 찾음
    (if _returnvalue_2
      (Class|BPIInteractable|Interact(Message) (.HitActor (Collision|BreakHitResult _outhit)) self) ; BPI에 Self Ref를 입력값으로 넣어줌\nBP_PickupActor가 꺼내서 사용함
    )))

(event Input|ActionEvents|InputActionLightAttack
  (params (Key :type Key%20Structure :default "None"))
  ;[0 0 0] 공격
  (:Pressed
    (if (Utilities|Enum|Equal(Enum) (Default|GetCurrentState (Variables|Default|GetStateManagerComp)) "Attacking") ; 1. 이미 공격 중일 땐 반복 공격 못하게
      (Variables|/Game/CombatSystem/Blueprints/Components/BP_CombatComp.BP_CombatComp_C|SetbIsAttackSaved? (Variables|Default|GetCombatComp) true) ; 이미 공격 진행 중이면 다음 공격을 위한 플래그 세움
      (else
        (CallFunction|AttackEvent) ; 2. 플래그 세워져있지 않으면 일단 첫 공격 실행
      ))))

(event Input|ActionEvents|InputActionDodge
  (params (Key :type Key%20Structure :default "None"))
  ;[0 0 0] 회피
  (:Pressed
    (CallFunction|DodgeEvent)))

(event Input|ActionEvents|InputActionToggleWalk
  (params (Key :type Key%20Structure :default "None"))
  (:Pressed
    (if (Utilities|Enum|NotEqual(Enum) (Class|RagnarokCharacter|GetCurrentSpeedMode) "Walking")
      (CallFunction|SetMovementSpeedMode "Walking")
      (else
        (CallFunction|SetMovementSpeedMode "Joging")))))

(event Input|ActionEvents|InputActionSprint
  (params (Key :type Key%20Structure :default "None"))
  (:Pressed
    (CallFunction|SetMovementSpeedMode "Sprinting"))
  (:Released
    (if (Utilities|Enum|Equal(Enum) (Class|RagnarokCharacter|GetCurrentSpeedMode) "Sprinting")
      (CallFunction|SetMovementSpeedMode "Joging"))))

(fn ConstructionScript)

(fn PerformAttack
  (params (CharacterAction :type ECharacterAction%20Enum :default "GeneralAction") (CharacterState :type ECharacterState%20Enum :default "GeneralActionState") (AttackIndex :type Integer) (bRandomIndex? :type Boolean))
  (bind _combatcomp (Variables|Default|GetCombatComp))
  (bind _combatcomp_2 (Variables|Default|GetCombatComp))
  (bind _mainweapon (Default|GetMainWeapon _combatcomp_2))
  (bind _attackmontages (Variables|/Game/CombatSystem/Blueprints/Actors/BP_BaseWeapon.BP_BaseWeapon_C|GetAttackMontages _mainweapon))
  (bind _output_get (LocalVariables|SetL_AttackMontage (select bRandomIndex? (.OutItem (Utilities|Array|Random _attackmontages)) (Utilities|Array|Get(acopy) _attackmontages AttackIndex)))) ; 5. 배열에 담겨있는 몽타주 중 선택된 하나
  (Utilities|IsValid _output_get
    (:Is%20Valid
      (Default|SetState (Variables|Default|GetStateManagerComp) CharacterState) ; 6. State 변경
      (Default|SetCurrentAction (Variables|Default|GetStateManagerComp) CharacterAction) ; LightAttack, ChargedAttack 등등
      (Animation|PlayAnimMontage (LocalVariables|GetL_AttackMontage) 1.0 "None") ; 7. 선택된 몽타주 재생
      (bind _result (Math|Integer|IncrementInt (Variables|/Game/CombatSystem/Blueprints/Components/BP_CombatComp.BP_CombatComp_C|GetAttackCount _combatcomp)) ; 8. 공격 횟수 카운트
        (:%20%20
          (if (> _result (Utilities|Array|LastIndex (Variables|/Game/CombatSystem/Blueprints/Actors/BP_BaseWeapon.BP_BaseWeapon_C|GetAttackMontages (Default|GetMainWeapon (Variables|Default|GetCombatComp))))) ; 9. 마지막 공격 콤보인가?
            (Variables|/Game/CombatSystem/Blueprints/Components/BP_CombatComp.BP_CombatComp_C|SetAttackCount _combatcomp 0) ; 10. 인덱스 초기화
          ))))))

(fn CanPerformToggleCombat?
  (return (and (not (Default|IsCurrentStateEqualtoAny? (Variables|Default|GetStateManagerComp) (Utilities|Array|MakeArray "Attacking" "Dodging" "Dead" "Disabled" "GeneralActionState"))) (not (AI|Components|NavMovement|IsFalling (Variables|Character|GetCharacterMovement))))))

(fn CanPerformAttack?
  (return (and (not (Default|IsCurrentStateEqualtoAny? (Variables|Default|GetStateManagerComp) (Utilities|Array|MakeArray "Attacking" "Dodging" "Dead" "Disabled" "GeneralActionState"))) (not (AI|Components|NavMovement|IsFalling (Variables|Character|GetCharacterMovement))))))

(fn CanPerformDodge?
  (return (and (not (Default|IsCurrentStateEqualtoAny? (Variables|Default|GetStateManagerComp) (Utilities|Array|MakeArray "Attacking" "Dodging" "Dead" "Disabled" "GeneralActionState"))) (not (AI|Components|NavMovement|IsFalling (Variables|Character|GetCharacterMovement))))))

(fn PerformDodge
  (params (MontageIndex :type Integer) (RandomIndex? :type Boolean))
  (bind _combatcomp (Variables|Default|GetCombatComp))
  (bind _mainweapon (Default|GetMainWeapon _combatcomp))
  (bind _dodgemontages (Variables|/Game/CombatSystem/Blueprints/Actors/BP_BaseWeapon.BP_BaseWeapon_C|GetDodgeMontages _mainweapon))
  (bind _output_get (LocalVariables|SetL_DodgeMontage (select RandomIndex? (.OutItem (Utilities|Array|Random _dodgemontages)) (Utilities|Array|Get(acopy) _dodgemontages (Math|Integer|SelectInt MontageIndex 0 (> MontageIndex (Utilities|Array|LastIndex (Variables|/Game/CombatSystem/Blueprints/Actors/BP_BaseWeapon.BP_BaseWeapon_C|GetDodgeMontages (Default|GetMainWeapon (Variables|Default|GetCombatComp)))))))))) ; 몽타주를 선택
  (Utilities|IsValid _output_get
    (:Is%20Valid
      (Default|SetState (Variables|Default|GetStateManagerComp) "Dodging") ; State 변경
      (Default|SetCurrentAction (Variables|Default|GetStateManagerComp) "Dodge")
      (Animation|PlayAnimMontage (LocalVariables|GetL_DodgeMontage) 1.0 "None") ; 선택된 몽타주 재생
    )))

(fn EnableRagdoll
  (bind _mesh (Variables|Character|GetMesh))
  (bind _pelvisbonename (Variables|Default|GetPelvisBoneName))
  (bind _capsulecomponent (Variables|Default|GetCapsuleComponent))
  (Pawn|Components|CharacterMovement|SetMovementMode (Variables|Character|GetCharacterMovement) "MOVE_None" 0) ; 이동불가
  (Collision|SetCollisionResponsetoChannel _capsulecomponent "ECC_Pawn" "ECR_Ignore") ; 캡슐 콜리전
  (Collision|SetCollisionResponsetoChannel _capsulecomponent "ECC_Camera" "ECR_Ignore") ; 캡슐 콜리전
  (Transformation|AttachComponentToComponent (Variables|Default|GetCameraBoom) (Variables|Character|GetMesh) (Variables|Default|GetPelvisBoneName) "KeepWorld" "KeepWorld" "KeepWorld" true) ; 카메라를 Pelvis로
  (Variables|/Script/Engine.SpringArmComponent|SetbDoCollisionTest (Variables|Default|GetCameraBoom) false) ; 카메라 콜리전 해제
  (Collision|SetCollisionProfileName _mesh "Ragdoll" true :!class /Script/Engine.PrimitiveComponent)
  (Class|SkeletalMeshComponent|SetAllBodiesBelowSimulatePhysics _mesh _pelvisbonename true true)
  (Class|SkeletalMeshComponent|SetAllBodiesBelowPhysicsBlendWeight _mesh _pelvisbonename 1.0 false true))

(fn ApplyHitReactionPhysicsVelocity
  (params (InitialSpeed :type Float%20%28double-precision%29))
  (Physics|SetPhysicsLinearVelocity (Variables|Character|GetMesh) (* (Transformation|GetActorForwardVector) (* InitialSpeed -1.0)) false (Variables|Default|GetPelvisBoneName)))

(fn CanJump?
  (return (and (not (Default|IsCurrentStateEqualtoAny? (Variables|Default|GetStateManagerComp) (Utilities|Array|MakeArray "Attacking" "Dodging" "Dead" "Disabled" "GeneralActionState"))) (not (AI|Components|NavMovement|IsFalling (Variables|Character|GetCharacterMovement))))))

(fn CanReceiveHitReaction?
  (return (not (Default|IsCurrentStateEqualtoAny? (Variables|Default|GetStateManagerComp) (Utilities|Array|MakeArray "Dead")))) ; Dead면 HitReaction 없게
)

(fn PerformAction
  (params (ActionMontages :type Array%20of%20Anim%20Montage%20Object%20References) (CharacterAction :type ECharacterAction%20Enum :default "GeneralAction") (CharacterState :type ECharacterState%20Enum :default "GeneralActionState") (MontageIndex :type Integer) (RandomIndex? :type Boolean))
  (bind _output_get (LocalVariables|SetL_DodgeMontage (select RandomIndex? (.OutItem (Utilities|Array|Random (Variables|/Game/CombatSystem/Blueprints/Actors/BP_BaseWeapon.BP_BaseWeapon_C|GetDodgeMontages (Default|GetMainWeapon (Variables|Default|GetCombatComp))))) (Utilities|Array|Get(acopy) ActionMontages (Math|Integer|SelectInt MontageIndex 0 (> MontageIndex (Utilities|Array|LastIndex (Variables|/Game/CombatSystem/Blueprints/Actors/BP_BaseWeapon.BP_BaseWeapon_C|GetDodgeMontages (Default|GetMainWeapon (Variables|Default|GetCombatComp)))))))))) ; 몽타주를 선택
  (Utilities|IsValid _output_get
    (:Is%20Valid
      (Default|SetState (Variables|Default|GetStateManagerComp) CharacterState) ; State 변경
      (Default|SetCurrentAction (Variables|Default|GetStateManagerComp) CharacterAction) ; Action 변경
      (Animation|PlayAnimMontage (LocalVariables|GetL_DodgeMontage) 1.0 "None") ; 선택된 몽타주 재생
    )))

(fn SetMovementSpeedMode
  (params (NewSpeedMode :type EMovementSpeedMode%20Enum :default "Walking"))
  (bind _charactermovement (Variables|Character|GetCharacterMovement))
  (if (Utilities|Enum|NotEqual(Enum) NewSpeedMode (Variables|Default|GetMovementSpeedMode))
    (bind _output_get (Variables|Default|SetMovementSpeedMode NewSpeedMode))
    (switch Utilities|FlowControl|Switch|SwitchonEMovementSpeedMode _output_get
      (:Walking
        (Variables|/Script/Engine.CharacterMovementComponent|SetMaxWalkSpeed _charactermovement (Variables|MovementSpeed|GetWalkingSpeed)))
      (:Joging
        (Variables|/Script/Engine.CharacterMovementComponent|SetMaxWalkSpeed _charactermovement (Variables|MovementSpeed|GetJoggingSpeed)))
      (:Sprinting
        (Variables|/Script/Engine.CharacterMovementComponent|SetMaxWalkSpeed _charactermovement (Variables|MovementSpeed|GetSprintingSpeed))))))

(fn CanReceiveDamage
  (return (Utilities|Enum|NotEqual(Enum) (Default|GetCurrentState (Variables|Default|GetStateManagerComp)) "Dead")))

(fn GetDesiredRotation
  (if (Utilities|Operators|NotEqual(!=) :A (Pawn|Components|PawnMovement|GetLastInputVector (Variables|Character|GetCharacterMovement)) :ErrorTolerance 0.001) ; 이동 입력 있냐?
    (return (Math|Conversions|RotationFromXVector (Class|Pawn|GetLastMovementInputVector))) ; 입력이 있으면 그 방향으로
    (else
      (return (Transformation|GetActorRotation)) ; 입력 없으면 현재 캐릭터 방향으로
    )))