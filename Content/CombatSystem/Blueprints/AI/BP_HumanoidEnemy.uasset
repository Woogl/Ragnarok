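; Humanoid enemy Blueprint for the combat system that adds a health bar shown according to its targeted state.
; On BeginPlay, it creates a WBP_HealthBar bound to its own StatsComp instead of the player's and assigns it to the HealthBar widget component.
; OnTargeted calls the parent handler, then sets the health bar's visibility to match the targeted flag.
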(event EventBeginPlay
  (|CallParentFunction)
  (bind _returnvalue (UserInterface|CreateWidget "/Game/CombatSystem/UI/WBP_HealthBar.WBP_HealthBar_C" (Game|GetPlayerController 0) (Variables|Default|GetStatsComp) false)) ; StatsComp를 WBP_HealthBar에 넘겨줌
  (UserInterface|SetWidget (Variables|Default|GetHealthBar) _returnvalue))

(event EventOnTargeted
  (params (bIsTargeted? :type Boolean))
  (|CallParentFunction bIsTargeted?)
  (Rendering|SetVisibility (Variables|Default|GetHealthBar) bIsTargeted? false))

(fn ConstructionScript
  (|CallParentFunction))