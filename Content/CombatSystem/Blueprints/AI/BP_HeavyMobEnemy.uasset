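; Heavy mob enemy Blueprint that extends a parent character with a melee weapon and a floating health bar.
; The health bar widget reads StatsComp and shows only while the enemy is targeted.
; Weapon collision hits apply stat-based point damage, and combat toggling moves the weapon mesh between hand and stowed sockets.
; On death, the weapon switches to the PhysicsActor collision profile, though SimulateWeaponPhysics sets physics simulation off.
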(event OnHit(MainWeaponCollisionComp)
  (params (HitResult :type Hit%20Result%20Structure))
  (bind _hitactor (Collision|BreakHitResult HitResult))
  (bind _returnvalue (Class|BPICombat|CanReceiveDamage(Message) _hitactor))
  (if _returnvalue
    (Game|Damage|ApplyPointDamage _hitactor (Default|GetCurrentStat (Variables|Default|GetStatsComp) "NewEnumerator4") (Transformation|GetActorForwardVector) HitResult (Pawn|GetController) self "/Game/CombatSystem/Blueprints/DamageTypes/BP_AttackDamageType.BP_AttackDamageType_C") ; CollisionTrace 맞은 놈에게에게 대미지
  ))

(event OnCombatToggle(CombatComp)
  (params (bIsCombatEnabled? :type Boolean))
  (Transformation|AttachComponentToComponent (Variables|Default|GetWeaponMesh) (Variables|Character|GetMesh) (select bIsCombatEnabled? (Variables|Initialization|GetWeaponHandSocket) (Variables|Initialization|GetAttachWeaponSocket)) "SnapToTarget" "SnapToTarget" "SnapToTarget" true))

(event Custom|SimulateWeaponPhysics
  (bind _weaponmesh (Variables|Default|GetWeaponMesh))
  (Collision|SetCollisionProfileName _weaponmesh "PhysicsActor" true :!class /Script/Engine.PrimitiveComponent)
  (Physics|SetSimulatePhysics _weaponmesh false))

(event EventBeginPlay
  (|CallParentFunction)
  (Default|SetCollisionMesh (Variables|Default|GetMainWeaponCollisionComp) (Variables|Default|GetWeaponMesh))
  (bind _returnvalue (UserInterface|CreateWidget "/Game/CombatSystem/UI/WBP_HealthBar.WBP_HealthBar_C" (Game|GetPlayerController 0) (Variables|Default|GetStatsComp) false)) ; StatsComp를 WBP_HealthBar에 넘겨줌
  (UserInterface|SetWidget (Variables|Default|GetHealthBar) _returnvalue))

(event EventPerformDeath
  (|CallParentFunction)
  (CallFunction|SimulateWeaponPhysics))

(event EventOnTargeted
  (params (bIsTargeted? :type Boolean))
  (|CallParentFunction bIsTargeted?)
  (Rendering|SetVisibility (Variables|Default|GetHealthBar) bIsTargeted? false))

(fn ConstructionScript
  (|CallParentFunction))