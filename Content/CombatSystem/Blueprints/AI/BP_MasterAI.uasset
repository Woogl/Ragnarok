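; Master AI enemy character for melee combat that attacks, reacts to hits, can be targeted and dies.
; Stats, combat, state-manager and weapon-collision components drive it, with gameplay tags selecting action montages and anim-notify messages chaining combos.
; Point damage reduces stats, reports to AI perception, spawns impact effects and plays front/back hit-stun or knockdown montages.
; State changes trigger timeline rotation toward the target when attacking, or ragdoll knockback and delayed destruction on death.
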(event OnStateBegin(StateManagerComp)
  (params (CharacterState :type Gameplay%20Tag%20Structure))
  ;[0 0 0] State
  (|SwitchGameplayTag CharacterState
    (:Character.State.Dead
      (CallFunction|PerformDeath))
    (:Character.State.Attacking
      (CallFunction|RotatetoTarget))))

(event OnStateEnd(StateManagerComp)
  (params (CharacterState :type Gameplay%20Tag%20Structure))
  ;[0 0 0] State
  (|SwitchGameplayTag CharacterState
    (:Character.State.Attacking
      (CallFunction|StopRotatingtoTarget))))

(event OnCombatToggle(CombatComp)
  (params (bIsCombatEnabled? :type Boolean)))

(event OnCurrentStatUpdate(StatsComp)
  (params (StatType :type E_Stats%20Enum :default "NewEnumerator0") (Value :type Float%20%28double-precision%29))
  ;[0 0 0] Stat Update
  (if (and (Utilities|Enum|Equal(Enum) StatType "NewEnumerator1") (<= Value 0.0)) ; 체력이 0 이하면 Dead 상태로
    (Default|SetState (Variables|Default|GetStateManagerComp) "(TagName=\"Character.State.Dead\")")))

(event Custom|AttackEvent
  ;[0 0 0] 공격
  (if (CallFunction|CanPerformAttack?)
    (if (Default|IsCombatEnabled? (Variables|Default|GetCombatComp))
      (CallFunction|PerformAttack (CallFunction|GetDesiredAttackType) (Variables|/Game/CombatSystem/Blueprints/Components/BP_CombatComp.BP_CombatComp_C|GetAttackCount (Variables|Default|GetCombatComp)) false))))

(event Custom|OnTargetSet
  (params (NewTarget :type Actor%20Object%20Reference))
  ;[0 0 0] 공격
  (Variables|Default|SetTargetActor NewTarget))

(event Custom|RotateToTarget
  (bind _returnvalue (Transformation|GetActorLocation))
  (bind _returnvalue_2 (Utilities|Time|GetWorldDeltaSeconds))
  (bind _returnvalue_3 (Transformation|GetActorRotation))
  (bind _targetactor (Variables|Default|GetTargetActor))
  (bind _returnvalue_4 (Transformation|GetActorLocation _targetactor))
  (bind _returnvalue_5 (Math|Rotator|FindLookatRotation _returnvalue _returnvalue_4))
  (bind _returnvalue_6 (Math|Interpolation|RInterpTo _returnvalue_3 _returnvalue_5 _returnvalue_2 9.0))
  ;[0 0 0] Rotate To Target
  (Timeline|TL_RotateToTarget PlayFromStart
    (:Update
      (Utilities|IsValid (Variables|Default|GetTargetActor)
        (:Is%20Valid
          (Transformation|SetActorRotation (Math|Rotator|MakeRotator (.Roll (Math|Rotator|BreakRotator _returnvalue_3)) (.pitch _returnvalue_6) (.yaw _returnvalue_6))))))))

(event Custom|StopRotatingToTarget
  (bind _returnvalue (Transformation|GetActorLocation))
  (bind _returnvalue_2 (Utilities|Time|GetWorldDeltaSeconds))
  (bind _returnvalue_3 (Transformation|GetActorRotation))
  (bind _targetactor (Variables|Default|GetTargetActor))
  (bind _returnvalue_4 (Transformation|GetActorLocation _targetactor))
  (bind _returnvalue_5 (Math|Rotator|FindLookatRotation _returnvalue _returnvalue_4))
  (bind _returnvalue_6 (Math|Interpolation|RInterpTo _returnvalue_3 _returnvalue_5 _returnvalue_2 9.0))
  ;[0 0 0] Rotate To Target
  (Timeline|TL_RotateToTarget Stop
    (:Update
      (Utilities|IsValid (Variables|Default|GetTargetActor)
        (:Is%20Valid
          (Transformation|SetActorRotation (Math|Rotator|MakeRotator (.Roll (Math|Rotator|BreakRotator _returnvalue_3)) (.pitch _returnvalue_6) (.yaw _returnvalue_6))))))))

(event Custom|PerformDeath
  ;[0 0 0] 사망
  (CallFunction|EnableRagdoll) ; 래그돌 일어나게
  (CallFunction|ApplyHitReactionPhysicsVelocity (select (Variables|Default|GetbHitFront?) 2e+03 -2e+03)) ; 캐릭터가 뒤로 밀리게
  (Utilities|FlowControl|Delay 4.0)
  (Actor|DestroyActor) ; 캐릭터 파괴
)

(event Custom|ApplyHitReaction
  (params (InDamageType :type E_DamageType%20Enum :default "NewEnumerator0"))
  ;[0 0 0] 피격 반응
  (switch Utilities|FlowControl|Switch|SwitchonE_DamageType InDamageType
    (:NewEnumerator0
      (CallFunction|PerformHitStun :!label _label))
    (:NewEnumerator1
      (goto _label))
    (:NewEnumerator2
      (CallFunction|PerformKnockdown))))

(event Custom|ApplyImpactEffect
  (params (DamageType :type E_DamageType%20Enum :default "NewEnumerator0"))
  (bind _lasthitinfo (Variables|Default|GetLastHitInfo))
  (bind _location (Collision|BreakHitResult _lasthitinfo))
  ;[0 0 0] 피격 반응
  (switch Utilities|FlowControl|Switch|SwitchonE_DamageType DamageType
    (:NewEnumerator1
      (Audio|PlaySoundatLocation "/Game/CombatSystem/CourseFiles/SoundFX/Gruntling/A_Guardian_Impact01_Cue.A_Guardian_Impact01_Cue" _location "0, 0, 0" 1.0 1.0 0.0 0 0 0 0) ; 타격 SFX
      (Effects|SpawnEmitteratLocation "/Game/VFX/Realistic_Starter_VFX_Pack_Vol2/Particles/Blood/P_Blood_Splat_Cone.P_Blood_Splat_Cone" _location) ; 타격 VFX
    )
    (:NewEnumerator2
      (Audio|PlaySoundatLocation "/Game/CombatSystem/CourseFiles/SoundFX/Gruntling/A_Guardian_Impact01_Cue.A_Guardian_Impact01_Cue" _location "0, 0, 0" 1.0 1.0 0.0 0 0 0 0) ; 타격 SFX
      (Effects|SpawnEmitteratLocation "/Game/VFX/Realistic_Starter_VFX_Pack_Vol2/Particles/Blood/P_Blood_Splat_Cone.P_Blood_Splat_Cone" _location) ; 타격 VFX
    )))

(event EventBeginPlay
  ;[0 0 0] Begin Play
  (Default|InitializeStat (Variables|Default|GetStatsComp)))

(event EventContinueAttack
  ;[0 0 0] Anim Notify 이벤트
  (if (Variables|/Game/CombatSystem/Blueprints/Components/BP_CombatComp.BP_CombatComp_C|GetbIsAttackSaved? (Variables|Default|GetCombatComp)) ; 다음 공격 입력했는지 플래그 체크
    (Variables|/Game/CombatSystem/Blueprints/Components/BP_CombatComp.BP_CombatComp_C|SetbIsAttackSaved? (Variables|Default|GetCombatComp) false) ; 플래그 초기화
    (if (== (Default|GetCurrentState (Variables|Default|GetStateManagerComp)) "(TagName=\"Character.State.Attacking\")") ; State 체크
      (Default|SetState (Variables|Default|GetStateManagerComp)))
    (CallFunction|AttackEvent) ; 다음 공격 콤보도 실행
  ))

(event EventSetiFrames
  (params (bEnableiFrames :type Boolean))
  ;[0 0 0] 피격 반응
  (Variables|Default|SetiFramesEnabled? bEnableiFrames))

(event EventResetAttack
  ;[0 0 0] Anim Notify 이벤트
  (Default|ResetAttack (Variables|Default|GetCombatComp)))

(event EventResetCombat
  ;[0 0 0] Anim Notify 이벤트
  (Default|ResetAttack (Variables|Default|GetCombatComp))
  (Default|ResetState (Variables|Default|GetStateManagerComp)) ; State를 Nothing으로 바꿈
  (Default|SetCurrentAction (Variables|Default|GetStateManagerComp)) ; Nothing
)

(event EventSetCanMove
  (params (bCanMove? :type Boolean))
  ;[0 0 0] BPI
  (Variables|Default|SetCan%20Move? bCanMove?))

(event Game|Damage|EventPointDamage
  (params (Damage :type Float%20%28single-precision%29) (DamageType :type Damage%20Type%20Object%20Reference) (HitLocation :type Vector :default "0, 0, 0") (HitNormal :type Vector :default "0, 0, 0") (HitComponent :type Primitive%20Component%20Object%20Reference) (BoneName :type Name :default "None") (ShotFromDirection :type Vector :default "0, 0, 0") (InstigatedBy :type Controller%20Object%20Reference) (DamageCauser :type Actor%20Object%20Reference) (HitInfo :type Hit%20Result%20Structure%20%28by%20ref%29))
  (bind _returnvalue (Pawn|GetControlledPawn InstigatedBy))
  ;[0 0 0] 피격
  (bind _asbp_attack_damage_type (Utilities|Casting|CastToBP_AttackDamageType DamageType))
  (Default|TakeDamage (Variables|Default|GetStatsComp) Damage)
  (Class|AISenseDamage|ReportDamageEvent self _returnvalue Damage HitLocation HitLocation "None") ; AI Perception에게 데미지 알림
  (Variables|Default|SetbHitFront? (Math|Float|InRange(Float) (Class|Actor|GetDotProductto self _returnvalue) 0.0 1.0)) ; 정면에서 맞았는지?
  (Variables|Default|SetLastHitInfo HitInfo)
  (CallFunction|ApplyImpactEffect (Variables|/Game/CombatSystem/Blueprints/DamageTypes/BP_AttackDamageType.BP_AttackDamageType_C|GetDamageType _asbp_attack_damage_type))
  (if (CallFunction|CanReceiveHitReaction?) ; Dead 상태는 HitReaction 없음
    (CallFunction|ApplyHitReaction (Variables|/Game/CombatSystem/Blueprints/DamageTypes/BP_AttackDamageType.BP_AttackDamageType_C|GetDamageType _asbp_attack_damage_type))))

(event EventMyJump
  ;[0 0 0] 점프
  (if (CallFunction|CanJump?)
    (Animation|StopAnimMontage 0) ; 재생 중이던 애니메이션 캔슬
    (Default|ResetState (Variables|Default|GetStateManagerComp))
    (Character|Jump)))

(event EventOnTargeted
  (params (bIsTargeted? :type Boolean))
  (Rendering|SetVisibility (Variables|Default|GetTargetingWidget) bIsTargeted? false))

(event EventActivateCollision
  (params (CollisionPart :type E_CollisionPart%20Enum :default "NewEnumerator0"))
  (Default|ActivateCollision (Variables|Default|GetMainWeaponCollisionComp)))

(event EventDeactivateCollision
  (params (CollisionPart :type E_CollisionPart%20Enum :default "NewEnumerator0"))
  (Default|DeactivateCollision (Variables|Default|GetMainWeaponCollisionComp)))

(event Input|KeyboardEvents|Tab
  (params (Key :type Key%20Structure :default "None"))
  ;[1 1 1] 디버그
  (:Pressed
    (Default|ModifyCurrentStat (Variables|Default|GetStatsComp) "NewEnumerator1" -25.0 true)))

(fn ConstructionScript)

(fn CanPerformToggleCombat?
  (return (and (not (Default|IsCurrentStateEqualtoAny? (Variables|Default|GetStateManagerComp) "(GameplayTags=((TagName=\"Character.State.Attacking\"),(TagName=\"Character.State.Dodging\"),(TagName=\"Character.State.Dead\"),(TagName=\"Character.State.Disabled\"),(TagName=\"Character.State.GeneralActionState\")))")) (not (AI|Components|NavMovement|IsFalling (Variables|Character|GetCharacterMovement))))))

(fn CanPerformAttack?
  (return (and (not (Default|IsCurrentStateEqualtoAny? (Variables|Default|GetStateManagerComp) "(GameplayTags=((TagName=\"Character.State.Dodging\"),(TagName=\"Character.State.Dead\"),(TagName=\"Character.State.Disabled\"),(TagName=\"Character.State.GeneralActionState\"),(TagName=\"Character.State.Attacking\")))")) (>= (Default|GetCurrentStat (Variables|Default|GetStatsComp) "NewEnumerator2") 1e+01))))

(fn CanPerformDodge?
  (return (Math|Boolean|ANDBoolean (not (Default|IsCurrentStateEqualtoAny? (Variables|Default|GetStateManagerComp) "(GameplayTags=((TagName=\"Character.State.Attacking\"),(TagName=\"Character.State.Dead\"),(TagName=\"Character.State.Disabled\"),(TagName=\"Character.State.Dodging\"),(TagName=\"Character.State.GeneralActionState\")))")) (not (AI|Components|NavMovement|IsFalling (Variables|Character|GetCharacterMovement))) (>= (Default|GetCurrentStat (Variables|Default|GetStatsComp) "NewEnumerator2") 1e+01))))

(fn EnableRagdoll
  (bind _mesh (Variables|Character|GetMesh))
  (bind _pelvisbonename (Variables|Default|GetPelvisBoneName))
  (bind _capsulecomponent (Variables|Default|GetCapsuleComponent))
  (Pawn|Components|CharacterMovement|SetMovementMode (Variables|Character|GetCharacterMovement) "MOVE_None" 0) ; 이동불가
  (Collision|SetCollisionResponsetoChannel _capsulecomponent "ECC_Pawn" "ECR_Ignore") ; 캡슐 콜리전
  (Collision|SetCollisionResponsetoChannel _capsulecomponent "ECC_Camera" "ECR_Ignore") ; 캡슐 콜리전
  (Collision|SetCollisionProfileName _mesh "Ragdoll" true :!class /Script/Engine.PrimitiveComponent)
  (Class|SkeletalMeshComponent|SetAllBodiesBelowSimulatePhysics _mesh _pelvisbonename true true)
  (Class|SkeletalMeshComponent|SetAllBodiesBelowPhysicsBlendWeight _mesh _pelvisbonename 1.0 false true))

(fn ApplyHitReactionPhysicsVelocity
  (params (InitialSpeed :type Float%20%28double-precision%29))
  (Physics|SetPhysicsLinearVelocity (Variables|Character|GetMesh) (* (Transformation|GetActorForwardVector) (* InitialSpeed -1.0)) false (Variables|Default|GetPelvisBoneName)))

(fn CanJump?
  (return (and (not (Default|IsCurrentStateEqualtoAny? (Variables|Default|GetStateManagerComp) "(GameplayTags=((TagName=\"Character.State.Attacking\"),(TagName=\"Character.State.Dead\"),(TagName=\"Character.State.Disabled\"),(TagName=\"Character.State.Dodging\"),(TagName=\"Character.State.GeneralActionState\")))")) (not (AI|Components|NavMovement|IsFalling (Variables|Character|GetCharacterMovement))))))

(fn CanReceiveHitReaction?
  (return (not (Default|IsCurrentStateEqualtoAny? (Variables|Default|GetStateManagerComp) "(GameplayTags=((TagName=\"Character.State.Dead\")))"))) ; Dead면 HitReaction 없게
)

(fn SetMovementSpeedMode
  (params (NewSpeedMode :type EMovementSpeedMode%20Enum :default "Walking"))
  (bind _charactermovement (Variables|Character|GetCharacterMovement))
  (if (Utilities|Enum|NotEqual(Enum) NewSpeedMode (Variables|Default|GetMovementSpeedMode))
    (bind _output_get (Variables|Default|SetMovementSpeedMode NewSpeedMode))
    (switch Utilities|FlowControl|Switch|SwitchonEMovementSpeedMode _output_get
      (:Walking
        (Variables|/Script/Engine.CharacterMovementComponent|SetMaxWalkSpeed _charactermovement (Variables|MovementSpeed|GetWalkingSpeed)))
      (:Joging
        (Variables|/Script/Engine.CharacterMovementComponent|SetMaxWalkSpeed _charactermovement (Variables|MovementSpeed|GetJoggingSpeed)))
      (:Sprinting
        (Variables|/Script/Engine.CharacterMovementComponent|SetMaxWalkSpeed _charactermovement (Variables|MovementSpeed|GetSprintingSpeed))))))

(fn GetDesiredAttackType
  (if (AI|Components|NavMovement|IsFalling (Variables|Character|GetCharacterMovement))
    (return "(TagName=\"Character.Action.Attack.FallingAttack\")")
    (elif (Utilities|Enum|Equal(Enum) (Class|RagnarokCharacter|GetCurrentSpeedMode) "Sprinting")
      (return "(TagName=\"Character.Action.Attack.SprintAttack\")")
      (else
        (return "(TagName=\"Character.Action.Attack.LightAttack\")")))))

(fn CanSprint?
  (return (!= (Math|Vector|VectorLength (Transformation|GetVelocity)) 0.0)))

(fn PerformHitStun
  (bind _output_get (LocalVariables|SetL_HitMontage (select (Variables|Default|GetbHitFront?) (Variables|Montages|HitReactions|GetHitStunFrontMontage) (Variables|Montages|HitReactions|GetHitStunBackMontage))))
  (Utilities|IsValid _output_get
    (:Is%20Valid
      (Default|SetState (Variables|Default|GetStateManagerComp) "(TagName=\"Character.State.Disabled\")") ; 이동 불가 상태
      (Animation|PlayAnimMontage (LocalVariables|GetL_HitMontage) 1.0 "None") ; 피격 모션
      (return true))
    (:Is%20Not%20Valid
      (return false))))

(fn PerformKnockdown
  (bind _output_get (LocalVariables|SetL_HitMontage (select (Variables|Default|GetbHitFront?) (Variables|Montages|HitReactions|GetKnockdownFrontMontage) (Variables|Montages|HitReactions|GetKnockdownBackMontage))))
  (Utilities|IsValid _output_get
    (:Is%20Valid
      (Default|SetState (Variables|Default|GetStateManagerComp) "(TagName=\"Character.State.Disabled\")") ; 이동 불가 상태
      (Animation|PlayAnimMontage (LocalVariables|GetL_HitMontage) 1.0 "None") ; 피격 모션
      (return true))
    (:Is%20Not%20Valid
      (return false))))

(fn GetActionMontage
  (params (ActionTag :type Gameplay%20Tag%20Structure))
  (|SwitchGameplayTag ActionTag
    (:Character.Action.Attack.CloseRange
      (return (Variables|Montages|Attacks|GetCloseRangeAttackMontages)))
    (:Character.Action.Dodge
      (return (Variables|Montages|Actions|GetDodgeMontages)))
    (:Character.Action.EnterCombat
      (return (Utilities|Array|MakeArray (Variables|Montages|Actions|GetEnterCombat))))
    (:Character.Action.ExitCombat
      (return (Utilities|Array|MakeArray (Variables|Montages|Actions|GetExitCombat))))
    (:Character.Action.Attack.MediumRange
      (return (Variables|Montages|Attacks|GetMediumRangeAttackMontages)))
    (:Character.Action.Attack.RareAttack
      (return (Variables|Montages|Attacks|GetRareAttackMontages)))))

(fn CanbeTargeted?
  (return (not (Default|IsCurrentStateEqualtoAny? (Variables|Default|GetStateManagerComp) "(GameplayTags=((TagName=\"Character.State.Dead\")))"))))

(fn CanReceiveDamage
  (return (and (not (Default|IsCurrentStateEqualtoAny? (Variables|Default|GetStateManagerComp) "(GameplayTags=((TagName=\"Character.State.Dead\")))")) (not (Variables|Default|GetiFramesEnabled?)))))

(fn GetDesiredRotation
  (if (Utilities|Operators|NotEqual(!=) :A (Pawn|Components|PawnMovement|GetLastInputVector (Variables|Character|GetCharacterMovement)) :ErrorTolerance 0.001) ; 이동 입력 있냐?
    (return (Math|Conversions|RotationFromXVector (Class|Pawn|GetLastMovementInputVector))) ; 입력이 있으면 그 방향으로
    (else
      (return (Transformation|GetActorRotation)) ; 입력 없으면 현재 캐릭터 방향으로
    )))

(fn GetMovementSpeedMode
  (return (Class|RagnarokCharacter|GetCurrentSpeedMode)))

(fn GetOwnedGameplayTags
  (return (Variables|GameplayTags|GetOwnedGameplayTags)))

(fn HasMatchingGameplayTags
  (params (TagToCheck :type Gameplay%20Tag%20Structure))
  (return (GameplayTags|HasTag (Variables|GameplayTags|GetOwnedGameplayTags) TagToCheck)))

(fn PerformAction
  (params (ActionTag :type Gameplay%20Tag%20Structure) (StateTag :type Gameplay%20Tag%20Structure) (MontageIndex :type Integer) (bRandomInex? :type Boolean))
  (LocalVariables|SetL_ActionMontages (CallFunction|GetActionMontage ActionTag)) ; 몽타주 목록 보관
  (bind _output_get (LocalVariables|SetL_ActionMontage (select bRandomInex? (.OutItem (Utilities|Array|Random (LocalVariables|GetL_ActionMontages))) (Utilities|Array|Get(acopy) (LocalVariables|GetL_ActionMontages) (select (> MontageIndex (Utilities|Array|LastIndex (LocalVariables|GetL_ActionMontages))) 0 MontageIndex))))) ; 몽타주를 선택
  (Utilities|IsValid _output_get
    (:Is%20Valid
      (Default|SetState (Variables|Default|GetStateManagerComp) StateTag) ; State 변경
      (Default|SetCurrentAction (Variables|Default|GetStateManagerComp) ActionTag) ; Action 변경
      (bind _returnvalue (Animation|Montage|MontagePlay (Components|SkeletalMesh|GetAnimInstance (Variables|Character|GetMesh)) (LocalVariables|GetL_ActionMontage) 1.0 "MontageLength" 0.0 true)) ; 선택된 몽타주 재생
      (return true _returnvalue))
    (:Is%20Not%20Valid
      (return false 0.0))))

(fn PerformAttack
  (params (AttackType :type Gameplay%20Tag%20Structure) (AttackIndex :type Integer) (bRandomInex? :type Boolean))
  (LocalVariables|SetL_AttackMontages (CallFunction|GetActionMontage AttackType)) ; 몽타주 목록 가져옴
  (bind _output_get (LocalVariables|SetL_AttackMontage (select bRandomInex? (.OutItem (Utilities|Array|Random (LocalVariables|GetL_AttackMontages))) (Utilities|Array|Get(acopy) (LocalVariables|GetL_AttackMontages) (select (> AttackIndex (Utilities|Array|LastIndex (LocalVariables|GetL_AttackMontages))) 0 AttackIndex))))) ; 배열에 담겨있는 몽타주 중 하나 선택
  (Utilities|IsValid _output_get
    (:Is%20Valid
      (Default|SetState (Variables|Default|GetStateManagerComp) "(TagName=\"Character.State.Attacking\")")
      (Default|SetCurrentAction (Variables|Default|GetStateManagerComp) AttackType) ; LightAttack, ChargedAttack 등등
      (bind _returnvalue (Animation|Montage|MontagePlay (Components|SkeletalMesh|GetAnimInstance (Variables|Character|GetMesh)) (LocalVariables|GetL_AttackMontage) 1.0 "MontageLength" 0.0 true)) ; 선택된 몽타주 재생
      (LocalVariables|SetL_AttackDuration _returnvalue)
      (bind _result (Math|Integer|IncrementInt (Variables|/Game/CombatSystem/Blueprints/Components/BP_CombatComp.BP_CombatComp_C|GetAttackCount (Variables|Default|GetCombatComp)))
        (:%20%20
          (if (> _result (Utilities|Array|LastIndex (LocalVariables|GetL_AttackMontages)))
            (Variables|/Game/CombatSystem/Blueprints/Components/BP_CombatComp.BP_CombatComp_C|SetAttackCount (Variables|Default|GetCombatComp) 0) ; 최대 콤보 넘었으면 초기화
          )
          (return true (LocalVariables|GetL_AttackDuration)))))
    (:Is%20Not%20Valid
      (Development|PrintString (Utilities|String|Append "Index: " (Utilities|String|ToString(Integer) AttackIndex) "is NOT VALID!"))
      (return false 0.0))))