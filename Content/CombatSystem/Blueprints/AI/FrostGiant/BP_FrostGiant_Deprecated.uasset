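; Deprecated Frost Giant boss Blueprint, extending a parent AI character with weapon combat and a boss health bar.
; Creates the health widget from its stats component on BeginPlay, toggling visibility with target acquisition and hiding it on death.
; Main weapon collision hits apply stat-based point damage to receptive actors, and combat toggles move the weapon between hand and attach sockets.
; Death switches the weapon to the PhysicsActor collision profile but leaves physics simulation off.
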(event OnHit(MainWeaponCollisionComp)
  (params (HitResult :type Hit%20Result%20Structure))
  (bind _hitactor (Collision|BreakHitResult HitResult))
  (bind _returnvalue (Class|BPICombat|CanReceiveDamage(Message) _hitactor))
  (if _returnvalue
    (Game|Damage|ApplyPointDamage _hitactor (Default|GetCurrentStat (Variables|Default|GetStatsComp) "NewEnumerator4") (Transformation|GetActorForwardVector) HitResult (Pawn|GetController) self "/Game/CombatSystem/Blueprints/DamageTypes/BP_AttackDamageType.BP_AttackDamageType_C") ; CollisionTrace 맞은 놈에게에게 대미지
  ))

(event OnCombatToggle(CombatComp)
  (params (bIsCombatEnabled? :type Boolean))
  (Transformation|AttachComponentToComponent (CallFunction|GetWeaponMesh) (Variables|Character|GetMesh) (select bIsCombatEnabled? (Variables|Initialization|GetWeaponHandSocket) (Variables|Initialization|GetAttachWeaponSocket)) "SnapToTarget" "SnapToTarget" "SnapToTarget" true))

(event Custom|SimulateWeaponPhysics
  (Collision|SetCollisionProfileName (CallFunction|GetWeaponMesh) "PhysicsActor" true :!class /Script/Engine.PrimitiveComponent)
  (Physics|SetSimulatePhysics (CallFunction|GetWeaponMesh) false))

(event Custom|SetBossHealthVisibility
  (params (bVisible? :type Boolean))
  (bind _bosshealthui (Variables|Default|GetBossHealthUI)
    (:then
      (Widget|SetVisibility _bosshealthui (select (and bVisible? (not (Default|IsCurrentStateEqualtoAny? (Variables|Default|GetStateManagerComp) "(GameplayTags=((TagName=\"Character.State.Dead\")))"))) "Visible" "Hidden")))
    (:else)))

(event EventBeginPlay
  (|CallParentFunction)
  (Default|SetCollisionMesh (Variables|Default|GetRightWeaponCollisionComp))
  (bind _returnvalue (UserInterface|CreateWidget "/Game/CombatSystem/UI/WBP_BossHealth.WBP_BossHealth_C" (Game|GetPlayerController 0)))
  (bind _output_get (Variables|Default|SetBossHealthUI _returnvalue))
  (Default|Initialize _output_get (Variables|Default|GetStatsComp))
  (UserInterface|Viewport|AddtoViewport (Variables|Default|GetBossHealthUI) 0))

(event EventPerformDeath
  (|CallParentFunction)
  (CallFunction|SimulateWeaponPhysics)
  (CallFunction|SetBossHealthVisibility false))

(event EventOnTargetSet
  (params (NewTarget :type Actor%20Object%20Reference))
  (|CallParentFunction NewTarget)
  (CallFunction|SetBossHealthVisibility (Utilities|IsValid NewTarget)))

(event EventOnTargeted
  (params (bIsTargeted? :type Boolean))
  (|CallParentFunction bIsTargeted?))

(fn ConstructionScript
  (|CallParentFunction))