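; Weapon hit-detection component that reports melee hits to its owner, such as BP_BaseWeapon, through an OnHit dispatcher.
; While collision is enabled, Tick runs a multi-sphere object trace between two sockets on the assigned mesh.
; Each actor fires OnHit only once per activation, because EnableCollision clears the already-hit list.
; An ignore list and getters expose trace state to other Blueprints.
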(event Custom|EnableCollision
  ;[0 0 0] Enable Collision
  (CallFunction|ClearHitActors)
  (Variables|Default|SetbIsCollisionEnabled? true))

(event Custom|DisableCollision
  ;[0 0 0] Disable Collision
  (Variables|Default|SetbIsCollisionEnabled? false))

(event Custom|CollisionTrace
  (bind _collisionmeshcomp (Variables|Default|GetCollisionMeshComp))
  ;[0 0 0] Collision Trace for Pawn
  (bind _outhits (Collision|MultiSphereTraceForObjects (Transformation|GetSocketLocation _collisionmeshcomp (Variables|Initialization|GetStartSocketName)) (Transformation|GetSocketLocation _collisionmeshcomp (Variables|Initialization|GetEndStartSocketName)) (Variables|Initialization|GetTraceRadius) (Variables|Initialization|GetCollisionObjectType) false (Variables|Default|GetActors%20to%20Ignore) "None"))
  (for _array_element _outhits
    (bind _output_get (Variables|Default|SetLastHit _array_element))
    (if (not (Utilities|Array|ContainsItem (Variables|Default|GetAlreadyHitActor) (.HitActor (Collision|BreakHitResult _output_get)))) ; 새로 맞은 적만 배열 넣음
      (bind _output_get_2 (Variables|Default|SetHit%20Actor (.HitActor (Collision|BreakHitResult _output_get))))
      (Utilities|Array|Add (Variables|Default|GetAlreadyHitActor) _output_get_2) ; 맞은 적에 추가
      (Default|CallOnHit (Variables|Default|GetLastHit)) ; Dispatcher Call -> BP_BaseWeapon
    )))

(event Custom|ClearHitActors
  ;[0 0 0] 맞은 적 초기화
  (Utilities|Array|Clear (Variables|Default|GetAlreadyHitActor)))

(event Custom|SetCollisionMesh
  (params (CollisionMeshComp :type Primitive%20Component%20Object%20Reference))
  ;[0 0 0] Set Collision Mesh
  (Variables|Default|SetCollisionMeshComp CollisionMeshComp))

(event EventTick
  (params (DeltaSeconds :type Float%20%28single-precision%29))
  ;[0 0 0] Tick
  (if (Variables|Default|GetbIsCollisionEnabled?)
    (CallFunction|CollisionTrace)))

(fn GetAlreadyHitActor
  (return (Variables|Default|GetAlreadyHitActor)))

(fn IsCollisionEnabled?
  (return (Variables|Default|GetbIsCollisionEnabled?)))

(fn GetLastHit
  (return (Variables|Default|GetLastHit)))

(fn GetCollisionMeshComp
  (return (Variables|Default|GetCollisionMeshComp)))

(fn AddActortoIgnore
  (params (InActor :type Actor%20Object%20Reference%20%28by%20ref%29))
  (Utilities|Array|AddUnique (Variables|Default|GetActors%20to%20Ignore) InActor))

(fn RemoveActortoIgnore
  (params (ActorToRemove :type Actor%20Object%20Reference%20%28by%20ref%29))
  (Utilities|Array|RemoveItem (Variables|Default|GetActors%20to%20Ignore) ActorToRemove))

(fn GetActorstoIgnore
  (return (Variables|Default|GetActors%20to%20Ignore)))