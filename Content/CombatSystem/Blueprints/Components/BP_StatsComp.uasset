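; Actor component that holds a combat character's stats, with base/max values in one map and current values in another.
; Every current-value write broadcasts an update dispatcher, and modifications clamp between zero and the stat's max.
; TakeDamage scales damage against Armor and sets the owner's state manager to Dead when Health runs out.
; Stamina changes flagged for regeneration restart a looping refill timer after a retriggerable delay, stopping at max.
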(event Custom|StartRegen
  (params (StatType :type E_Stats%20Enum :default "NewEnumerator0"))
  (switch Utilities|FlowControl|Switch|SwitchonE_Stats StatType
    (:NewEnumerator2
      (Utilities|Time|ClearTimerbyFunctionName 0 "RegenStamina") ; 잠시 리젠 타이머 멈춤
      (Utilities|FlowControl|RetriggerableDelay (Variables|Default|GetRegenDelay))
      (Utilities|Time|SetTimerbyFunctionName 0 "RegenStamina" 0.1 true) ; 다시 리젠 타이머 시작
    )))

(event EventBeginPlay)

(event EventTick
  (params (DeltaSeconds :type Float%20%28single-precision%29)))

(fn InitializeStat
  (bind _keys (Utilities|Map|Keys (Variables|BaseStats|GetBaseStats))) ; Map의 모든 key 값들을 반환
  (for _array_element _keys
    (CallFunction|SetCurrentStat _array_element (.basevalue (.Value (Utilities|Map|Find (Variables|BaseStats|GetBaseStats) _array_element))))))

(fn SetCurrentStat
  (params (Stat :type E_Stats%20Enum :default "NewEnumerator0") (Value :type Float%20%28double-precision%29))
  (Utilities|Map|Add (Variables|Default|GetCurrentStats) Stat Value)
  (Default|CallOnCurrentStatUpdate Stat Value) ; Event Dispatcher
)

(fn GetCurrentStat
  (params (Stat :type E_Stats%20Enum :default "NewEnumerator0"))
  (return (.Value (Utilities|Map|Find (Variables|Default|GetCurrentStats) Stat))))

(fn ModifyCurrentStat
  (params (Stat :type E_Stats%20Enum :default "NewEnumerator0") (Value :type Float%20%28double-precision%29) (bShouldRegenerate? :type Boolean))
  (if (!= Value 0.0)
    (bind _output_get (LocalVariables|SetL_Value (+ (CallFunction|GetCurrentStat Stat) Value)))
    (CallFunction|SetCurrentStat Stat (Math|Float|Clamp(Float) _output_get 0.0 (BaseStats|GetMaxStat Stat)))
    (if bShouldRegenerate?
      (CallFunction|StartRegen Stat))))

(fn GetMaxStat
  (params (Key :type E_Stats%20Enum :default "NewEnumerator0"))
  (return (.maxvalue (.Value (Utilities|Map|Find (Variables|BaseStats|GetBaseStats) Key)))))

(fn SetMaxStat
  (params (Stat :type E_Stats%20Enum :default "NewEnumerator0") (Value :type Float%20%28double-precision%29))
  (bind _structout (Utilities|Struct|SetmembersinF_BaseStat (.Value (Utilities|Map|Find (Variables|BaseStats|GetBaseStats) Stat)) Value)) ; Copy한 것의 Ref를 건드리는거라 진짜 원본 BaseStat은 그대로
  (Utilities|Map|Add (Variables|BaseStats|GetBaseStats) Stat _structout) ; 진짜 원본 BaseStat을 건드리게 함
)

(fn GetBaseStat
  (params (Key :type E_Stats%20Enum :default "NewEnumerator0"))
  (return (.basevalue (.Value (Utilities|Map|Find (Variables|BaseStats|GetBaseStats) Key)))))

(fn SetBaseStat
  (params (Stat :type E_Stats%20Enum :default "NewEnumerator0") (Value :type Float%20%28double-precision%29))
  (bind _structout (Utilities|Struct|SetmembersinF_BaseStat (.Value (Utilities|Map|Find (Variables|BaseStats|GetBaseStats) Stat)) Value)) ; Copy한 것의 Ref를 건드리는거라 진짜 원본 BaseStat은 그대로
  (Utilities|Map|Add (Variables|BaseStats|GetBaseStats) Stat _structout) ; 진짜 원본 BaseStat을 건드리게 함
)

(fn TakeDamage
  (params (InDamage :type Float%20%28double-precision%29))
  (bind _value (CallFunction|GetCurrentStat "NewEnumerator3"))
  (bind _returnvalue (+ InDamage _value))
  (bind _returnvalue_2 (/ InDamage _returnvalue))
  (bind _returnvalue_3 (* InDamage _returnvalue_2))
  (LocalVariables|SetL_Damage (Math|Float|Clamp(Float) _returnvalue_3 0.0 _returnvalue_3))
  (CallFunction|ModifyCurrentStat "NewEnumerator1" (* (LocalVariables|GetL_Damage) -1.0) true)
  (if (<= (CallFunction|GetCurrentStat "NewEnumerator1") 0.0) ; 체력 0 이하면 사망
    (Default|SetState (Actor|GetComponentbyClass (Components|GetOwner) "/Game/CombatSystem/Blueprints/Components/BP_StateManagerComp.BP_StateManagerComp_C") "(TagName=\"Character.State.Dead\")")))

(fn RegenStamina
  (CallFunction|SetCurrentStat "NewEnumerator2" (Math|Float|Clamp(Float) (+ (CallFunction|GetCurrentStat "NewEnumerator2") (Variables|Default|GetStaminaRegenRate)) 0.0 (BaseStats|GetMaxStat "NewEnumerator2")))
  (if (>= (CallFunction|GetCurrentStat "NewEnumerator2") (BaseStats|GetMaxStat "NewEnumerator2"))
    (Utilities|Time|ClearTimerbyFunctionName 0 "RegenStamina")))