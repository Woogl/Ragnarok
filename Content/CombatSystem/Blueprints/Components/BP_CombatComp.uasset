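; Combat component that holds a character's combat state: main weapon, equipped shield, combat mode, blocking and attack combo.
; Setting a main weapon unequips and destroys the previous one before storing the new one, while the shield setter only stores its reference.
; Combat and blocking changes broadcast event dispatchers, with blocking computed as the input compared unequal to the current state.
; ResetAttack clears the combo count and saved-attack flag, and no Tick logic runs.
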(event EventBeginPlay)

(event EventTick
  (params (DeltaSeconds :type Float%20%28single-precision%29)))

(fn SetMainWeapon
  (params (NewWeapon :type BP%20Base%20Weapon%20Object%20Reference))
  (Utilities|FlowControl|Sequence
    (:then_0
      (Utilities|IsValid (Variables|Default|GetMainWeapon)
        (:Is%20Valid
          (Default|OnUnequipped (Variables|Default|GetMainWeapon))
          (Actor|DestroyActor (Variables|Default|GetMainWeapon)) ; 기존 장착 무기 있으면 파괴
        )))
    (:then_1
      (Variables|Default|SetMainWeapon NewWeapon) ; 새 무기 지정
    )))

(fn GetMainWeapon
  (return (Variables|Default|GetMainWeapon)))

(fn SetCombatEnabled
  (params (Enabled? :type Boolean))
  (bind _output_get (Variables|Default|SetbCombatEnabled? Enabled?))
  (Default|CallOnCombatToggle _output_get))

(fn IsCombatEnabled?
  (return (Variables|Default|GetbCombatEnabled?)))

(fn ResetAttack
  (Variables|Default|SetAttackCount 0) ; 콤보 초기화
  (Variables|Default|SetbIsAttackSaved? false))

(fn SetBlockingState
  (params (bEnableBlocking? :type Boolean))
  (bind _output_get (Variables|Default|SetbIsBlocking (!= bEnableBlocking? (Variables|Default|GetbIsBlocking))))
  (Default|CallOnBlockingSet _output_get) ; Event Dispatcher
)

(fn SetShieldWeapon
  (params (InShield :type BP%20Base%20Weapon%20Object%20Reference))
  (Variables|Default|SetEquippedShield InShield))

(fn GetEquippedShield
  (return (Variables|Default|GetEquippedShield)))