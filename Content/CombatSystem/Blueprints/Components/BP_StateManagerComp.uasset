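; State manager component for the combat system, tracking its owner's current state and current character action as gameplay tags.
; Setters ignore unchanged values, otherwise firing an End dispatcher for the old value and a Begin dispatcher for the new one.
; Query functions test either value against a tag container by exact match, and ResetState sets the state back to the default tag.
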(event EventBeginPlay)

(event EventTick
  (params (DeltaSeconds :type Float%20%28single-precision%29)))

(fn SetState
  (params (NewState :type Gameplay%20Tag%20Structure))
  (if (!= NewState (Variables|Default|GetCurrentState))
    (Default|CallOnStateEnd (Variables|Default|GetCurrentState)) ; Event Dispatcher
    (Variables|Default|SetCurrentState NewState) ; C++ Enum
    (Default|CallOnStateBegin NewState) ; Event Dispatcher
  ))

(fn GetCurrentState
  (return (Variables|Default|GetCurrentState)))

(fn ResetState
  (CallFunction|SetState))

(fn IsCurrentStateEqualtoAny?
  (params (StatesToCheck :type Gameplay%20Tag%20Container%20Structure))
  (return (GameplayTags|HasTag StatesToCheck (Variables|Default|GetCurrentState) true)))

(fn SetCurrentAction
  (params (NewAction :type Gameplay%20Tag%20Structure))
  (if (!= NewAction (Variables|Default|GetCurrentAction))
    (Default|CallOnCharacterActionEnd (Variables|Default|GetCurrentAction)) ; Event Dispatcher
    (bind _output_get (Variables|Default|SetCurrentAction NewAction))
    (Default|CallOnCharacterActionBegin _output_get) ; Event Dispatcher
  ))

(fn GetCurrentAction
  (return (Variables|Default|GetCurrentAction)))

(fn IsCurrentActionEqualtoAny?
  (params (ActionsToCheck :type Gameplay%20Tag%20Container%20Structure))
  (return (GameplayTags|HasTag ActionsToCheck (Variables|Default|GetCurrentAction) true)))