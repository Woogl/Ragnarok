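; BP_MasterPose is an equippable item for skeletal armor pieces that follow the owning character's pose and change its armor stat.
; AttachActor overrides attachment: if the item's skeletal mesh is valid, it snaps it to a socket on the owner's character mesh and sets that mesh as master pose component.
; OnEquipped and OnUnequipped call their parents, then add or subtract ArmorValue through the owner's BP_StatsComp.
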(event EventBeginPlay
  (|CallParentFunction) ; This node is disabled and will not be called.\nDrag off pins to build functionality.
)

(event Collision|EventActorBeginOverlap
  (params (OtherActor :type Actor%20Object%20Reference))
  (|CallParentFunction OtherActor) ; This node is disabled and will not be called.\nDrag off pins to build functionality.
)

(event EventTick
  (params (DeltaSeconds :type Float%20%28single-precision%29))
  (|CallParentFunction DeltaSeconds) ; This node is disabled and will not be called.\nDrag off pins to build functionality.
)

(fn ConstructionScript
  (|CallParentFunction))

(fn AttachActor
  (params (SocketName :type Name :default "None"))
  (bind _returnvalue (Components|GetOwner))
  (bind _ascharacter (Utilities|Casting|CastToCharacter _returnvalue))
  (bind _mesh (Variables|/Script/Engine.Character|GetMesh _ascharacter))
  (Utilities|IsValid (Variables|/Script/Engine.SkinnedMeshComponent|GetSkeletalMesh (Variables|Default|GetItemSkeletalMesh))
    (:Is%20Valid
      (Transformation|AttachComponentToComponent (Variables|Default|GetItemSkeletalMesh) _mesh SocketName "SnapToTarget" "SnapToTarget" "SnapToTarget" true) ; 캐릭터 메쉬의 소켓에 붙임
      (Class|SkinnedMeshComponent|SetMasterPoseComponent (Variables|Default|GetItemSkeletalMesh) _mesh false) ; 붙어있는 메쉬의 포즈를 따라가게 함
      (return))
    (:Is%20Not%20Valid
      (return) ; 탈출
    )))

(fn OnEquipped
  (|CallParentFunction)
  (Default|ModifyCurrentStat (Actor|GetComponentbyClass (Components|GetOwner) "/Game/CombatSystem/Blueprints/Components/BP_StatsComp.BP_StatsComp_C") "NewEnumerator3" (Variables|Default|GetArmorValue) false) ; 방어력 상승
)

(fn OnUnequipped
  (|CallParentFunction)
  (Default|ModifyCurrentStat (Actor|GetComponentbyClass (Components|GetOwner) "/Game/CombatSystem/Blueprints/Components/BP_StatsComp.BP_StatsComp_C") "NewEnumerator3" (* (Variables|Default|GetArmorValue) -1.0) false) ; 방어력 하락
)