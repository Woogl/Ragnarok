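; BP_BaseEquippable is the abstract base actor for equippable combat items, such as swords, that attach to a character.
; OnEquipped sets the equipped flag and snaps the item to AttachSocket on the owning Character's mesh, with child Blueprints specifying the socket.
; OnUnequipped only clears the flag, without detaching.
; GetItemMesh returns the static mesh component if it has a mesh assigned, otherwise the skeletal one.
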(event EventBeginPlay)

(event Collision|EventActorBeginOverlap
  (params (OtherActor :type Actor%20Object%20Reference)))

(event EventTick
  (params (DeltaSeconds :type Float%20%28single-precision%29)))

(fn ConstructionScript)

(fn GetItemMesh
  (bind _itemstaticmesh (Variables|Default|GetItemStaticMesh))
  (Utilities|IsValid (Variables|/Script/Engine.StaticMeshComponent|GetStaticMesh _itemstaticmesh)
    (:Is%20Valid
      (return _itemstaticmesh))
    (:Is%20Not%20Valid
      (return (Variables|Default|GetItemSkeletalMesh)))))

(fn OnEquipped
  (CallFunction|SetIsEquipped true)
  (ItemMesh|AttachActor (Variables|Initialization|GetAttachSocket)))

(fn OnUnequipped
  (if (Variables|Default|GetbIsEquipped?)
    (Variables|Default|SetbIsEquipped? false)))

(fn AttachActor
  (params (SocketName :type Name))
  (Transformation|AttachComponentToComponent (Variables|/Script/Engine.Character|GetMesh (.AsCharacter (Utilities|Casting|CastToCharacter (Components|GetOwner)))) SocketName "SnapToTarget" "SnapToTarget" "SnapToTarget" true) ; 이놈이 무한 호출됨...
)

(fn SetIsEquipped
  (params (IsEquipped? :type Boolean))
  (Variables|Default|SetbIsEquipped? IsEquipped?))

(fn IsEquipped?
  (return (Variables|Default|GetbIsEquipped?)))