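; Base dual-wield weapon that extends BP_BaseWeapon with an off-hand weapon and a right-foot attack.
; On equip and combat toggle, it attaches the off-hand mesh to a hand or stowed socket on the owner's character mesh.
; Activate/DeactivateCollision overrides route by collision part to main, off-hand or foot trace components.
; Off-hand and foot traces ignore the owner and apply point damage to hit actors that can receive it.
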(event OnHit(OffHandWeaponCollisionComp)
  (params (HitResult :type Hit%20Result%20Structure))
  (bind _hitactor (Collision|BreakHitResult HitResult))
  (bind _returnvalue (Class|BPICombat|CanReceiveDamage(Message) _hitactor))
  (if _returnvalue
    (Game|Damage|ApplyPointDamage _hitactor (CallFunction|GetDamage) (Transformation|GetActorForwardVector (Components|GetOwner)) HitResult (Game|GetInstigatorController) self) ; CollisionTrace 맞은 놈에게에게 대미지
  ))

(event OnHit(RightFootCollisionComp)
  (params (HitResult :type Hit%20Result%20Structure))
  (bind _hitactor (Collision|BreakHitResult HitResult))
  (bind _returnvalue (Class|BPICombat|CanReceiveDamage(Message) _hitactor))
  (if _returnvalue
    (Game|Damage|ApplyPointDamage _hitactor (CallFunction|GetDamage) (Transformation|GetActorForwardVector (Components|GetOwner)) HitResult (Game|GetInstigatorController) self) ; CollisionTrace 맞은 놈에게에게 대미지
  ))

(event EventBeginPlay
  (|CallParentFunction) ; This node is disabled and will not be called.\nDrag off pins to build functionality.
)

(event Collision|EventActorBeginOverlap
  (params (OtherActor :type Actor%20Object%20Reference))
  (|CallParentFunction OtherActor) ; This node is disabled and will not be called.\nDrag off pins to build functionality.
)

(event EventTick
  (params (DeltaSeconds :type Float%20%28single-precision%29))
  (|CallParentFunction DeltaSeconds) ; This node is disabled and will not be called.\nDrag off pins to build functionality.
)

(event EventToggleCombat
  (params (bEnableCombat :type Boolean))
  (|CallParentFunction bEnableCombat) ; SetCombatEnabled / AttachActor\n첫번째 무기
  (CallFunction|AttachOff-HandWeapon (select bEnableCombat (Variables|Initialization|GetSecondWeaponHandSocket) (Variables|Initialization|GetSecondWeaponAttachSocket))) ; 두번째 무기
)

(fn ConstructionScript
  (|CallParentFunction))

(fn ActivateCollision
  (params (CollisionPart :type E_CollisionPart%20Enum :default "NewEnumerator0"))
  (switch Utilities|FlowControl|Switch|SwitchonE_CollisionPart CollisionPart
    (:NewEnumerator0
      (Default|ActivateCollision (Variables|Default|GetMainWeaponCollisionComp)))
    (:NewEnumerator1
      (Default|ActivateCollision (Variables|Default|GetOffHandWeaponCollisionComp)))
    (:NewEnumerator2
      (Default|ActivateCollision (Variables|Default|GetRightFootCollisionComp)))))

(fn DeactivateCollision
  (params (CollisionPart :type E_CollisionPart%20Enum :default "NewEnumerator0"))
  (switch Utilities|FlowControl|Switch|SwitchonE_CollisionPart CollisionPart
    (:NewEnumerator0
      (Default|DeactivateCollision (Variables|Default|GetMainWeaponCollisionComp)))
    (:NewEnumerator1
      (Default|DeactivateCollision (Variables|Default|GetOffHandWeaponCollisionComp)))
    (:NewEnumerator2
      (Default|DeactivateCollision (Variables|Default|GetRightFootCollisionComp)))))

(fn OnEquipped
  (|CallParentFunction)
  (Default|SetCollisionMesh (Variables|Default|GetOffHandWeaponCollisionComp) (Variables|Default|GetOffHandWeaponMesh))
  (Default|SetCollisionMesh (Variables|Default|GetRightFootCollisionComp) (Variables|/Script/Engine.Character|GetMesh (.AsCharacter (Utilities|Casting|CastToCharacter (Components|GetOwner)))))
  (CallFunction|AttachOff-HandWeapon (select (Default|IsCombatEnabled? (Variables|Default|GetOwnerCombatComp)) (Variables|Initialization|GetSecondWeaponHandSocket) (Variables|Initialization|GetSecondWeaponAttachSocket)))
  (Default|AddActortoIgnore (Variables|Default|GetOffHandWeaponCollisionComp) (Components|GetOwner)) ; 자기 자신은 못때리게
  (Default|AddActortoIgnore (Variables|Default|GetRightFootCollisionComp) (Components|GetOwner)) ; 자기 자신은 못때리게
)

(fn AttachOff-HandWeapon
  (params (Socket :type Name))
  (Transformation|AttachComponentToComponent (Variables|Default|GetOffHandWeaponMesh) (Variables|/Script/Engine.Character|GetMesh (.AsCharacter (Utilities|Casting|CastToCharacter (Components|GetOwner)))) Socket "SnapToTarget" "SnapToTarget" "SnapToTarget" true))