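; BP_BaseWeapon is the base equippable weapon of the combat system, handling attachment, hit damage and montage lookup.
; On equip it attaches to the hand or stow socket by combat state, registers with BP_CombatComp, sends its combat type to the owner's AnimInstance and sets up CollisionComp, ignoring the owner.
; CollisionComp hits deal point damage to actors that can receive it.
; GetActionMontages maps each character action to the weapon's montages.
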(event OnHit(CollisionComp)
  (params (HitResult :type Hit%20Result%20Structure))
  (bind _hitactor (Collision|BreakHitResult HitResult))
  (bind _returnvalue (Class|BPICombat|CanReceiveDamage(Message) _hitactor))
  (if _returnvalue
    (Game|Damage|ApplyPointDamage _hitactor (Variables|Default|GetDamage) (Transformation|GetActorForwardVector (Components|GetOwner)) HitResult (Game|GetInstigatorController) self) ; CollisionTrace 맞은 놈에게에게 대미지
  ))

(event Custom|SimulateWeaponPhysics
  (bind _newparam (CallFunction|GetItemMesh))
  (Collision|SetCollisionProfileName _newparam "PhysicsActor" true :!class /Script/Engine.PrimitiveComponent)
  (Physics|SetSimulatePhysics _newparam false))

(event EventBeginPlay
  (|CallParentFunction) ; This node is disabled and will not be called.\nDrag off pins to build functionality.
)

(event Collision|EventActorBeginOverlap
  (params (OtherActor :type Actor%20Object%20Reference))
  (|CallParentFunction OtherActor) ; This node is disabled and will not be called.\nDrag off pins to build functionality.
)

(event EventTick
  (params (DeltaSeconds :type Float%20%28single-precision%29))
  (|CallParentFunction DeltaSeconds) ; This node is disabled and will not be called.\nDrag off pins to build functionality.
)

(fn ConstructionScript
  (|CallParentFunction))

(fn OnEquipped
  (|CallParentFunction)
  (CallFunction|SetIsEquipped true)
  (Variables|Default|SetCombatComponent (Actor|GetComponentbyClass (Components|GetOwner) "/Game/CombatSystem/Blueprints/Components/BP_CombatComp.BP_CombatComp_C"))
  (CallFunction|AttachActor (select (Default|IsCombatEnabled? (Variables|Default|GetCombatComponent)) (Variables|Initialization|GetHandSocketName) (Variables|Default|GetAttachSocketName)))
  (Default|SetMainWeapon (Variables|Default|GetCombatComponent) self)
  (Class|BPIAnimInstance|UpdateCombatType(Message) (Components|SkeletalMesh|GetAnimInstance (Variables|/Script/Engine.Character|GetMesh (.AsCharacter (Utilities|Casting|CastToCharacter (Components|GetOwner))))) (Variables|Initialization|GetCombatType)) ; Interface에 값 넣어줌
  (Default|SetCollisionMesh (Variables|Default|GetCollisionComp) (CallFunction|GetItemMesh))
  (Default|AddActortoIgnore (Variables|Default|GetCollisionComp) (Components|GetOwner)) ; 자기 자신은 못때리게
)

(fn GetActionMontages
  (params (CharacterAction :type ECharacterAction%20Enum :default "Nothing"))
  (return (Utilities|Select :Index CharacterAction :Nothing 0 :General 0 :LightAttack (Variables|Montages|GetLightAttackMontages) :HeavyAttack (Variables|Montages|GetHeavyAttackMontages) :ChargedAttack (Variables|Montages|GetChargedAttackMontages) :FallingAttack (Variables|Montages|GetFallingAttacks) :Dodge (Variables|Montages|GetDodgeMontages) :EnterCombat (Utilities|Array|MakeArray (Variables|Montages|GetEnterCombat)) :ExitCombat (Utilities|Array|MakeArray (Variables|Montages|GetExitCombat)))))