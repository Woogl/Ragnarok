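; BP_BaseShield is the base shield equippable for the combat system, with attach sockets left to child Blueprints.
; On equip it caches the owner's combat, state and stats components, binds to combat toggling and attaches to the hand or stowed socket.
; It registers as the shield weapon, sends its combat type to the AnimInstance and sets up owner-ignoring collision.
; OnEquipped replaces the parent logic, while OnUnequipped extends it by clearing the shield slot.
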(event EventBeginPlay
  (|CallParentFunction) ; This node is disabled and will not be called.\nDrag off pins to build functionality.
)

(event Collision|EventActorBeginOverlap
  (params (OtherActor :type Actor%20Object%20Reference))
  (|CallParentFunction OtherActor) ; This node is disabled and will not be called.\nDrag off pins to build functionality.
)

(event EventTick
  (params (DeltaSeconds :type Float%20%28single-precision%29))
  (|CallParentFunction DeltaSeconds) ; This node is disabled and will not be called.\nDrag off pins to build functionality.
)

(fn ConstructionScript
  (|CallParentFunction))

(fn OnEquipped
  (CallFunction|SetIsEquipped true)
  (CallFunction|AttachActor (Variables|Default|GetAttachSocket))
  (bind _output_get (Variables|Default|SetOwnerCombatComp (Actor|GetComponentbyClass (Components|GetOwner) "/Game/CombatSystem/Blueprints/Components/BP_CombatComp.BP_CombatComp_C")))
  (EventDispatchers|BindEventtoOnCombatToggle _output_get (EventDispatchers|CreateEvent :!event ToggleWeaponCombat))
  (Variables|Default|SetOwnerStateManagerComp (Actor|GetComponentbyClass (Components|GetOwner) "/Game/CombatSystem/Blueprints/Components/BP_StateManagerComp.BP_StateManagerComp_C"))
  (Variables|Default|SetOwnerStatsComp (Actor|GetComponentbyClass (Components|GetOwner) "/Game/CombatSystem/Blueprints/Components/BP_StatsComp.BP_StatsComp_C"))
  (CallFunction|AttachActor (select (Default|IsCombatEnabled? (Variables|Default|GetOwnerCombatComp)) (Variables|Default|GetHandSocket) (Variables|Default|GetAttachSocket)))
  (Default|SetShieldWeapon (Variables|Default|GetOwnerCombatComp) self) ; 부모와 다른 부분
  (Class|BPIAnimInstance|UpdateCombatType(Message) (Components|SkeletalMesh|GetAnimInstance (Variables|/Script/Engine.Character|GetMesh (.AsCharacter (Utilities|Casting|CastToCharacter (Components|GetOwner))))) (Variables|Default|GetCombatType)) ; Interface에 값 넣어줌
  (Default|SetCollisionMesh (Variables|Default|GetMainWeaponCollisionComp) (CallFunction|GetItemMesh))
  (Default|AddActortoIgnore (Variables|Default|GetMainWeaponCollisionComp) (Components|GetOwner)) ; 자기 자신은 못때리게
)

(fn OnUnequipped
  (|CallParentFunction)
  (Default|SetShieldWeapon (Variables|Default|GetOwnerCombatComp)) ; 방패 없음
)